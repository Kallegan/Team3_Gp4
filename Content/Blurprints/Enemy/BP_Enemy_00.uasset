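; BP_Enemy_00 is an enemy actor that loses a hitpoint whenever the player begins overlapping its HitCollider.
; It registers itself on BeginPlay by incrementing EnemyCount in BP_GameMode.
; When its hitpoints run out, it decrements that count, calls CheckEnemyCount on the game mode and destroys itself.
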(event `self.ReceiveBeginPlay`
  ;[1 1 1] Add enemy count to game instance
  (bind _asbp_game_mode (cast `/Game/Blurprints/BP_GameMode` (`GameplayStatics.GetGameMode`)))
  (bind _result (`/Engine/EditorBlueprintResources/StandardMacros.IncrementInt` (`/Game/Blurprints/BP_GameMode.EnemyCount` _asbp_game_mode))
    (:`  `
      (set `/Game/Blurprints/BP_GameMode.EnemyCount` _result _asbp_game_mode))))

(event `self.Hit Collider.OnComponentBeginOverlap`
  (params (OverlappedComponent :type "PrimitiveComponent Object Reference") (OtherActor :type "Actor Object Reference") (OtherComp :type "PrimitiveComponent Object Reference") (OtherBodyIndex :type Integer) (bFromSweep :type Boolean) (SweepResult :type "HitResult Structure (by ref)"))
  ;[1 1 1] Enemy take damage and is removed from enemy count
  (cast `/Game/Blurprints/Player/BP_Player` OtherActor)
  (set `self.Hitpoints` (- (`self.Hitpoints`) 1))
  (if (<= (`self.Hitpoints`) 0)
    (bind _asbp_game_mode (cast `/Game/Blurprints/BP_GameMode` (`GameplayStatics.GetGameMode`)))
    (bind _result (`/Engine/EditorBlueprintResources/StandardMacros.DecrementInt` (`/Game/Blurprints/BP_GameMode.EnemyCount` _asbp_game_mode))
      (:`  `
        (set `/Game/Blurprints/BP_GameMode.EnemyCount` _result _asbp_game_mode)
        (`/Game/Blurprints/BP_GameMode.CheckEnemyCount` _asbp_game_mode)
        (`self.K2_DestroyActor`)))))

(fn `UserConstructionScript`)