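; BP_Player is a player Blueprint that moves a physics Sphere, with movement and camera controls marked as temporary.
; MoveForward and MoveRight inputs call MoveActor, which pushes the Sphere with a force along the Camera's forward or right vector, scaled by MoveForce.
; Look inputs pass through a CameraRotation helper into controller pitch and yaw.
; The helper's sensitivity and delta-time scaling appears unconnected.
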(event `InputAxis|MoveForward`
  (params (AxisValue :type "Float (single-precision)"))
  ;[1 1 1] temp basic movement
  (`self.MoveActor` AxisValue (`SceneComponent.GetForwardVector` (`self.Camera`))))

(event `InputAxis|MoveRight`
  (params (AxisValue :type "Float (single-precision)"))
  ;[1 1 1] temp basic movement
  (`self.MoveActor` AxisValue (`SceneComponent.GetRightVector` (`self.Camera`))))

(event `InputAxis|LookUp`
  (params (AxisValue :type "Float (single-precision)"))
  ;[1 1 1] temp basic camera
  (`self.AddControllerPitchInput` (`self.CameraRotation` AxisValue)))

(event `InputAxis|LookRight`
  (params (AxisValue :type "Float (single-precision)"))
  ;[1 1 1] temp basic camera
  (`self.AddControllerYawInput` (`self.CameraRotation` AxisValue)))

(fn `MoveActor`
  (params (B :type "Float (single-precision)") (MoveDirection :type "Vector Structure"))
  (`PrimitiveComponent.AddForce` (`self.Sphere`) (* B (* (* MoveDirection (`self.MoveForce`)) (100.0 100.0 100.0))) "None" false))

(fn `UserConstructionScript`)